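; Game mode Blueprint for Attack mode that places players at start positions matched to the player count.
; On BeginPlay it binds to the game start event, which then runs SetPlayerStartPositions.
; That function matches each player to a PlayerStart tagged with player count and one-based player number (e.g. 3_2), then moves the existing pawn to its location, leaving rotation untouched.
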(event `self.ReceiveBeginPlay`
  (add `self.OnGameStart` (delegate `OnGameStartImpl`)))

(event `OnGameStartImpl`
  (`self.SetPlayerStartPositions`))

(fn `SetPlayerStartPositions`
  (locals (PlayerStartActors :type "Array of PlayerStart Object Reference"))
  (bind _outactors (`GameplayStatics.GetAllActorsOfClass` "/Script/Engine.PlayerStart"))
  (set `local.PlayerStartActors` _outactors)
  (bind _returnvalue (`self.GetNumPlayers`))
  (for _index (range (+ _returnvalue 1))
    (for _array_element (`local.PlayerStartActors`)
      (bind _index_2 (`/Game/Blueprints/TetrisGlobals.GetPlayerIndex` (`GameplayStatics.GetPlayerController` _index)))
      (if (`KismetStringLibrary.EqualEqual_StrStr` (`KismetStringLibrary.Conv_NameToString` (`PlayerStart.PlayerStartTag` _array_element)) (`KismetTextLibrary.Conv_TextToString` (`|FormatText` "{NumPlayers}_{PlayerID}" _returnvalue (+ _index_2 1))))
        (`self.K2_SetActorLocation` (`GameplayStatics.GetPlayerPawn` _index_2) (`self.K2_GetActorLocation` _array_element) false false)))))

(fn `UserConstructionScript`)