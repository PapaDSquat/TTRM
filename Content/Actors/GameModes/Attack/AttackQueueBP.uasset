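; AttackQueueBP is an actor in the Attack game mode that displays a queue as up to eight block components.
; SetBlockNum shows the first Num blocks and hides the rest, looking up each by index through GetBlockComponent.
; SetBlockTheme is an empty stub, and the event graph and construction script contain no logic.
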(event `self.ReceiveBeginPlay`)

(fn `GetBlockComponent`
  (params (Num :type Integer))
  (returns (Component :type "ChildActorComponent Object Reference"))
  (switch `int` Num
    (:`Default`
      (return null))
    (:`1`
      (return (`self.Block1`)))
    (:`2`
      (return (`self.Block2`)))
    (:`3`
      (return (`self.Block3`)))
    (:`4`
      (return (`self.Block4`)))
    (:`5`
      (return (`self.Block5`)))
    (:`6`
      (return (`self.Block6`)))
    (:`7`
      (return (`self.Block7`)))
    (:`8`
      (return (`self.Block8`)))))

(fn `SetBlockNum`
  (params (Num :type Integer))
  (for _index (range 1 9)
    (`SceneComponent.SetHiddenInGame` (`self.GetBlockComponent` _index) (> _index Num) false)))

(fn `SetBlockTheme`)

(fn `UserConstructionScript`)