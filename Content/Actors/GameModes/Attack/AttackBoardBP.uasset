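; AttackBoardBP is a board actor for the Attack game mode that displays its pawn's attack queue size.
; On BeginPlay it subscribes to AttackGameModeBP's queue-changed and game-start events.
; Queue changes whose source matches the board's pawn, and a reset to zero at game start, feed SetQueueNum, which sets the block count on its AttackQueueBP child actor.
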(event `self.ReceiveBeginPlay`
  (bind _gamemode (`self.GetAttackGameMode`))
  (`parent.ReceiveBeginPlay`)
  (add `AttackGameMode.OnQueueChanged` _gamemode (delegate `OnQueueChanged`))
  (add `TetrisGameMode.OnGameStart` _gamemode (delegate `OnGameStart_Event_0`)))

(event `OnQueueChanged`
  (params (NewQueueSize :type Integer) (Source :type "PlayerPawn Object Reference"))
  (if (== Source (`self.GetPawn`))
    (`self.SetQueueNum` NewQueueSize)))

(event `OnGameStart_Event_0`
  (`self.SetQueueNum` 0))

(fn `GetAttackGameMode`
  (returns (GameMode :type "/Game/GameModes/AttackGameModeBP Object Reference"))
  (bind _asattack_game_mode_bp (cast `/Game/GameModes/AttackGameModeBP` (`self.GameMode`))
    (:`then`
      _)
    (:`CastFailed`
      _))
  (return _asattack_game_mode_bp))

(fn `SetQueueNum`
  (params (Num :type Integer))
  (bind _asattack_queue_bp (cast `/Game/Actors/GameModes/Attack/AttackQueueBP` (`ChildActorComponent.ChildActor` (`self.AttackQueueBP`))))
  (`/Game/Actors/GameModes/Attack/AttackQueueBP.SetBlockNum` _asattack_queue_bp Num))

(fn `UserConstructionScript`
  (`parent.UserConstructionScript`))