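; Background actor for the Tetris game that restyles its cube's material when the game theme changes.
; The construction script creates and stores a dynamic instance of the background material on the cube.
; On BeginPlay it subscribes to the Tetris game mode's theme change event, then applies the theme's background parameters to that instance whenever it fires, along with a debug print.
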(event `self.ReceiveBeginPlay`
  (bind _astetris_game_mode (cast `TetrisGameMode` (`GameplayStatics.GetGameMode`)))
  (bind _output_get (set `self.GameMode` _astetris_game_mode))
  ;[1 1 1] Set Material Texture
  (add `TetrisGameMode.OnThemeChange` _output_get (delegate `OnThemeChange`)))

(event `OnThemeChange`
  (params (Theme :type "TetrisTheme Structure (by ref)"))
  ;[1 1 1] Set Material Texture
  (`/Game/Blueprints/TetrisGlobals.SetThemeMaterialParams` (`self.DMI`) Theme_BackgroundTheme)
  (`KismetSystemLibrary.PrintString` "Hello"))

(fn `UserConstructionScript`
  (bind _returnvalue (`PrimitiveComponent.CreateDynamicMaterialInstance` (`self.Cube`) 0 "/Game/Themes/GuardianSoft/Material/GS_Material_BG.GS_Material_BG"))
  (set `self.DMI` _returnvalue))