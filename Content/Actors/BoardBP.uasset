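; Tetris board actor that shows the themed border and back, plus text readouts of the owning player's level, lines and score.
; Construction creates dynamic materials for both meshes, which update from the game mode's current theme and its theme-change event.
; Tick polls round stats from the owner pawn's PlayerState to refresh the text, a step marked as better event-based.
; SetUIVisible shows or hides the whole text hierarchy.
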(event `self.ReceiveBeginPlay`
  (bind _astetris_game_mode (cast `TetrisGameMode` (`GameplayStatics.GetGameMode`)))
  (bind _output_get (set `self.GameMode` _astetris_game_mode))
  (`|ExecutionSequence`
    (:`then_0`
      ;[1 1 1] Set Theme
      (add `TetrisGameMode.OnThemeChange` _output_get (delegate `OnThemeChange`))
      (`self.OnThemeChange` (`TetrisGameMode.GetCurrentTheme` _output_get)) ; Set initial theme
    )))

(event `OnThemeChange`
  (params (Theme :type "TetrisTheme Structure (by ref)"))
  ;[1 1 1] Set Theme
  (`/Game/Blueprints/TetrisGlobals.SetThemeMaterialParams` (`self.BorderDMI`) Theme_BorderTheme)
  (`/Game/Blueprints/TetrisGlobals.SetThemeMaterialParams` (`self.BackBMI`) Theme_BackTheme))

(event `self.ReceiveTick`
  (params (DeltaSeconds :type "Float (single-precision)"))
  (`self.UpdateUI`) ; Should be event-based
)

(fn `GetPawn`
  (returns (OwnerPawn :type "/Game/Player/PlayerPawnBP Object Reference"))
  (bind _asplayer_pawn_bp (cast `/Game/Player/PlayerPawnBP` (`self.GetOwner`))
    (:`then`
      _)
    (:`CastFailed`
      _))
  (return _asplayer_pawn_bp))

(fn `GetPlayerState`
  (returns (PlayerState :type "TetrisPlayerState Object Reference"))
  (bind _astetris_player_state (cast `TetrisPlayerState` (`Pawn.PlayerState` (`self.GetPawn`)))
    (:`then`
      _)
    (:`CastFailed`
      _))
  (return _astetris_player_state))

(fn `SetUIVisible`
  (params (Visible :type Boolean))
  (`SceneComponent.SetHiddenInGame` (`self.TextRoot`) (not Visible) true))

(fn `UpdateUI`
  (bind _playerstate (`self.GetPlayerState`))
  (bind (_returnvalue_score _returnvalue_lines _returnvalue_level) (break `PlayerRoundStats` (`TetrisPlayerState.GetRoundStats` _playerstate)))
  (bind (_returnvalue_score_2 _returnvalue_lines_2) (break `PlayerRoundStats` (`TetrisPlayerState.GetRoundStats` _playerstate)))
  (bind _returnvalue_score_3 (break `PlayerRoundStats` (`TetrisPlayerState.GetRoundStats` _playerstate)))
  (`|ExecutionSequence`
    (:`then_0`
      (`TextRenderComponent.K2_SetText` (`self.Text_Level_Value`) (`KismetTextLibrary.Conv_IntToText` _returnvalue_level false false)))
    (:`then_1`
      (`TextRenderComponent.K2_SetText` (`self.Text_Lines_Value`) (`KismetTextLibrary.Conv_IntToText` _returnvalue_lines_2 false false)))
    (:`then_2`
      (`TextRenderComponent.K2_SetText` (`self.Text_Score_Value`) (`KismetTextLibrary.Conv_IntToText` _returnvalue_score_3 false false)))))

(fn `UserConstructionScript`
  (bind _returnvalue (`PrimitiveComponent.CreateDynamicMaterialInstance` (`self.Border`) 0 "/Game/Themes/Common/Material_Border.Material_Border" "None"))
  (set `self.BorderDMI` _returnvalue)
  (bind _returnvalue_2 (`PrimitiveComponent.CreateDynamicMaterialInstance` (`self.Back`) 0 "/Game/Themes/Common/Material_Back.Material_Back" "None"))
  (set `self.BackBMI` _returnvalue_2))