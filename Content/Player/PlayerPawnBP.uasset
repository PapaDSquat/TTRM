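; Player pawn Blueprint for a Tetris game that manages the pause and game-over menus.
; On BeginPlay it creates both menus and binds to the TetrisGameMode's game start and game over events, which hide or show the game-over screen.
; SetGamePaused, driven by game start and Pause input, calls the GameMode and toggles cursor and pause menu.
; HUD creation, per-player positioning and board UI toggling are disconnected.
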(event `self.ReceiveBeginPlay`
  (bind _gamemode (`self.GameMode`))
  (bind _astetris_game_mode (cast `TetrisGameMode` (`GameplayStatics.GetGameMode`)))
  (set `self.GameMode` _astetris_game_mode)
  (`|ExecutionSequence`
    (:`then_1`
      (bind _returnvalue (`|CreateWidget` "/Game/UI/Menus/PauseMenu.PauseMenu_C"))
      (set `self.PauseMenu` _returnvalue))
    (:`then_2`
      (bind _returnvalue_2 (`|CreateWidget` "/Game/UI/Menus/GameOverMenu.GameOverMenu_C"))
      (set `self.GameOverMenu` _returnvalue_2))
    (:`then_3`
      (add `TetrisGameMode.OnGameStart` _gamemode (delegate `OnGameStart`)))
    (:`then_4`
      (add `TetrisGameMode.OnGameOver` _gamemode (delegate `OnGameOver`)))))

(event `OnGameStart`
  (`Widget.RemoveFromParent` (`self.GameOverMenu`))
  (`self.SetGamePaused` false))

(event `OnGameOver`
  (`Widget.RemoveFromParent` (`self.PlayerHUD`))
  (`UserWidget.AddToViewport` (`self.GameOverMenu`) 0))

(event `InputAction|Pause`
  (params (Key :type "Key Structure"))
  (:`Pressed`
    (`self.SetGamePaused` (not (`self.Paused`)))))

(fn `GetBoardBP`
  (returns (BoardBP :type "/Game/Actors/BoardBP Object Reference"))
  (bind _asboard_bp (cast `/Game/Actors/BoardBP` (`self.GetBoard`))
    (:`then`
      _)
    (:`CastFailed`
      _))
  (return _asboard_bp))

(fn `SetGamePaused`
  (params (paused :type Boolean))
  (bind _pausemenu (`self.PauseMenu`))
  (bind _gamemode (`self.GameMode`))
  (bind _output_get (set `self.Paused` paused))
  (if _output_get
    (`TetrisGameMode.PauseGame` _gamemode)
    (else
      (`TetrisGameMode.UnpauseGame` _gamemode)))
  (bind _output_get_2 (set `PlayerController.bShowMouseCursor` _output_get (`GameplayStatics.GetPlayerController` 0)))
  (if _output_get_2
    (`UserWidget.AddToViewport` _pausemenu 0)
    (else
      (`Widget.RemoveFromParent` _pausemenu))))

(fn `UserConstructionScript`)